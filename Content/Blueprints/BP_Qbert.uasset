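; BP_Qbert is a keyboard-controlled character, apparently a Q*bert, that moves in hops along the X and Y axes.
; W, A, S and D each add a fixed, mass-dependent impulse to CharacterMovement, with W and A launching higher than S and D.
; The cast that stores a BP_TheConstructor reference is never executed, and SpawnLocation and the construction script are empty.
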(event `Key|S`
  (params (Key :type "Key Structure"))
  (:`Pressed`
    (`CharacterMovementComponent.AddImpulse` (`self.CharacterMovement`) (0.0 100.0 400.0) false)))

(event `Key|W`
  (params (Key :type "Key Structure"))
  (:`Pressed`
    (`CharacterMovementComponent.AddImpulse` (`self.CharacterMovement`) (0.0 -100.0 500.0) false)))

(event `Key|D`
  (params (Key :type "Key Structure"))
  (:`Pressed`
    (`CharacterMovementComponent.AddImpulse` (`self.CharacterMovement`) (100.0 -0.0 400.0) false)))

(event `Key|A`
  (params (Key :type "Key Structure"))
  (:`Pressed`
    (`CharacterMovementComponent.AddImpulse` (`self.CharacterMovement`) (-100.0 0.0 500.0) false)))

(fn `SpawnLocation`)

(fn `UserConstructionScript`)