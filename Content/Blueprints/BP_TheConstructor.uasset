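; Constructor actor that procedurally builds a stepped Q*bert-style block pyramid on BeginPlay from a configurable step count.
; It spawns a root pyramid and four face actors, each yawed a further 90 degrees and attached to the root.
; Each face gets diagonal rows of blocks, shrinking by one per level, with KeepRelative attachment carrying them into the face's rotation.
; It also computes a Qbert spawn transform above the apex.
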(event `self.ReceiveBeginPlay`
  (bind _returnvalue (+ (* (`self.Dynamic Step Count`) -100.0) 50.0))
  (set `self.Static Step Count` (`self.Dynamic Step Count`))
  ;[1 1 1] Creates the ofset for origin
  (`self.Qbert Spawner Location Generator`)
  ;;[1 0 0] Pyramid Spawn
  (bind _returnvalue_2 (`|SpawnActorFromClass` "/Game/Blueprints/BP_Pyramid.BP_Pyramid_C" (`self.Origin`) "Undefined" "OverrideRootScale" null null))
  (`self.EnableInput` (`GameplayStatics.GetPlayerController` 0))
  (for _ (range 4)
    (set `self.Dynamic Step Count` (`self.Static Step Count`))
    (set `self.Block Spawn` (`KismetMathLibrary.MakeTransform` (`KismetMathLibrary.MakeVector` _returnvalue 50.0)))
    (set `self.Block Spawn Location X` _returnvalue)
    ;[1 0.08229 0.08229] Face Spawn
    (bind _returnvalue_3 (`|SpawnActorFromClass` "/Game/Blueprints/BP_PyramidFace.BP_PyramidFace_C" (`self.Origin`) "Undefined" "OverrideRootScale" null null))
    (bind _output_get (set `self.FaceCount` (+ (`self.FaceCount`) 1)))
    (`self.K2_AddActorLocalRotation` _returnvalue_3 (`KismetMathLibrary.MakeRotator` 0.0 0.0 (`KismetMathLibrary.Conv_IntToDouble` (* (`self.FaceCount`) 90))) false false)
    (`self.K2_AttachToActor` _returnvalue_3 _returnvalue_2 "None" "KeepRelative" "KeepRelative" "KeepRelative" true)
    (set `self.Dynamic Step Count` (`self.Static Step Count`))
    (set `self.Height` 0.0)
    (while (> (`self.Dynamic Step Count`) 0)
      (set `self.Count` 0)
      (while (< (`self.Count`) (`self.Dynamic Step Count`))
        ;[1 0.2781 0.2781] Block Spawn
        (`self.CreateBlock` _returnvalue_3)
        (set `self.Count` (+ (`self.Count`) 1)))
      (set `self.Block Spawn` (`KismetMathLibrary.MakeTransform` (`KismetMathLibrary.MakeVector` (+ (`self.Height`) (+ (`self.Block Spawn Location X`) 100.0)) 50.0 (+ (.z (.location (`self.Block Spawn`))) 100.0))))
      (set `self.Dynamic Step Count` (- (`self.Dynamic Step Count`) 1))
      (set `self.Height` (+ (`self.Height`) 100.0))
      (set `self.Count` 0))
    (`KismetSystemLibrary.PrintString` (`KismetStringLibrary.Conv_IntToString` _output_get))))

(fn `CreateBlock`
  (params (ParentActor :type "Actor Object Reference"))
  (bind _block_spawn_location (`KismetMathLibrary.BreakTransform` (`self.Block Spawn`)))
  (bind _returnvalue (`|SpawnActorFromClass` "/Game/Blueprints/BP_PyramidBlock.BP_PyramidBlock_C" (`self.Block Spawn`) "AlwaysSpawn" "OverrideRootScale" null null))
  (set `self.Block Spawn` (`KismetMathLibrary.MakeTransform` (+ _block_spawn_location (100.0 100.0 0.0))))
  (`self.K2_AttachToActor` _returnvalue ParentActor "None" "KeepRelative" "KeepRelative" "KeepRelative" true))

(fn `Qbert Spawner Location Generator`
  (set `self.QbertLocation` (`KismetMathLibrary.MakeTransform` (`KismetMathLibrary.MakeVector` -50.0 50.0 (`KismetMathLibrary.Conv_IntToDouble` (+ (* (`self.Dynamic Step Count`) 100) 100))))))

(fn `UserConstructionScript`)