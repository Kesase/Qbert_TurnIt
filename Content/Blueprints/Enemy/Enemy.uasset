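; Snake enemy for a Q*bert-style game that chases the player character in grid hops.
; Tick records its Y and Z, then four delayed branches compare them with the player's stored position to pick a diagonal direction.
; Each hop sets the facing and moves the capsule in two offset steps, up-then-across or across-then-down.
; KeyFree clears on moves and resets after capsule hits, but never gates movement.
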(event `self.CapsuleComponent.OnComponentHit`
  (params (HitComponent :type "PrimitiveComponent Object Reference") (OtherActor :type "Actor Object Reference") (OtherComp :type "PrimitiveComponent Object Reference") (NormalImpulse :type "Vector Structure") (Hit :type "HitResult Structure (by ref)"))
  (`KismetSystemLibrary.Delay` 0.15)
  (set `self.Key Free` true))

(event `self.ReceiveBeginPlay`
  (bind _asthird_person_character (cast `/Game/Blueprints/ThirdPersonCharacter` (`GameplayStatics.GetPlayerCharacter` 0)))
  (set `self.As Third Person Character` _asthird_person_character))

(event `self.ReceiveTick`
  (params (DeltaSeconds :type "Float (single-precision)"))
  (bind (_returnvalue_x _returnvalue_y _returnvalue_z) (`KismetMathLibrary.BreakVector` (`self.K2_GetActorLocation`)))
  (bind _capsulecomponent (`self.CapsuleComponent`))
  (bind _capsulecomponent_2 (`self.CapsuleComponent`))
  (bind _capsulecomponent_3 (`self.CapsuleComponent`))
  (bind _capsulecomponent_4 (`self.CapsuleComponent`))
  (`|ExecutionSequence`
    (:`then_0`
      (set `self.Snake Left Or Right` _returnvalue_y)
      (set `self.Snake Highness` _returnvalue_z))
    (:`then_1`
      (`KismetSystemLibrary.Delay` 1.0)
      (if (and (>= (`self.Snake Left Or Right`) (`/Game/Blueprints/ThirdPersonCharacter.Qbert Left Or Right` (`self.As Third Person Character`))) (>= (`/Game/Blueprints/ThirdPersonCharacter.Qbert Highness` (`self.As Third Person Character`)) (`self.Snake Highness`)))
        (set `self.Key Free` false)
        (`self.K2_SetActorRotation` (struct :`Yaw` 270.0))
        (`SceneComponent.K2_AddRelativeLocation` _capsulecomponent_2 (0.0 0.0 100.0) false false)
        (`KismetSystemLibrary.Delay` 0.2)
        (`SceneComponent.K2_AddRelativeLocation` _capsulecomponent_2 (0.0 -100.0 0.0) false false)))
    (:`then_2`
      (`KismetSystemLibrary.Delay` 1.0)
      (if (and (>= (`/Game/Blueprints/ThirdPersonCharacter.Qbert Left Or Right` (`self.As Third Person Character`)) (`self.Snake Left Or Right`)) (>= (`self.Snake Highness`) (`/Game/Blueprints/ThirdPersonCharacter.Qbert Highness` (`self.As Third Person Character`))))
        (set `self.Key Free` false)
        (`self.K2_SetActorRotation` (struct :`Yaw` 90.0))
        (`SceneComponent.K2_AddRelativeLocation` _capsulecomponent_3 (0.0 100.0 0.0) false false)
        (`KismetSystemLibrary.Delay` 0.2)
        (`SceneComponent.K2_AddRelativeLocation` _capsulecomponent_3 (0.0 0.0 -100.0) false false)))
    (:`then_3`
      (`KismetSystemLibrary.Delay` 1.0)
      (if (and (>= (`/Game/Blueprints/ThirdPersonCharacter.Qbert Left Or Right` (`self.As Third Person Character`)) (`self.Snake Left Or Right`)) (>= (`/Game/Blueprints/ThirdPersonCharacter.Qbert Highness` (`self.As Third Person Character`)) (`self.Snake Highness`)))
        (set `self.Key Free` false)
        (`self.K2_SetActorRotation` (struct :`Yaw` 360.0))
        (`SceneComponent.K2_AddRelativeLocation` _capsulecomponent_4 (0.0 0.0 100.0) false false)
        (`KismetSystemLibrary.Delay` 0.2)
        (`SceneComponent.K2_AddRelativeLocation` _capsulecomponent_4 (100.0 0.0 0.0) false false)))
    (:`then_4`
      (`KismetSystemLibrary.Delay` 1.0)
      (if (and (>= (`self.Snake Highness`) (`/Game/Blueprints/ThirdPersonCharacter.Qbert Highness` (`self.As Third Person Character`))) (>= (`self.Snake Left Or Right`) (`/Game/Blueprints/ThirdPersonCharacter.Qbert Left Or Right` (`self.As Third Person Character`))))
        (set `self.Key Free` false)
        (`self.K2_SetActorRotation` (struct :`Yaw` 180.0))
        (`SceneComponent.K2_AddRelativeLocation` _capsulecomponent (-100.0 0.0 0.0) false false)
        (`KismetSystemLibrary.Delay` 0.2)
        (`SceneComponent.K2_AddRelativeLocation` _capsulecomponent (0.0 0.0 -100.0) false false)))))

(fn `UserConstructionScript`)