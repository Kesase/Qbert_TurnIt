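; LevelCamera is a level camera that places itself at a fixed, angled vantage point and sizes its orthographic view at BeginPlay.
; BeginPlay proceeds only if an Options cast succeeds, then sets the ortho width and the actor transform.
; CameraLocationAndValueGenerator computes that width linearly from a BP_TheConstructor class default.
; Perspective/orthographic switching based on Options.PersOrOrth exists but is disconnected, and Tick is empty.
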(event `self.ReceiveBeginPlay`
  (bind _asoptions (cast `/Game/MainMenu/Options` (`self.User WİD`)))
  (set `self.As Options` _asoptions)
  (bind _output_get (`self.Camera Location and Value Generator`))
  (`CameraComponent.SetOrthoWidth` (`self.CameraComponent`) _output_get)
  (`self.K2_SetActorTransform` (`KismetMathLibrary.MakeTransform` (-850.0 850.0 850.0) (struct :`Pitch` 330.0 :`Yaw` 315.0))))

(event `self.ReceiveTick`
  (params (DeltaSeconds :type "Float (single-precision)")))

(fn `Camera Location and Value Generator`
  (returns (Output_Get :type "Float (double-precision)"))
  (bind _asbp_the_constructor (castclass `/Game/Blueprints/BP_TheConstructor` "/Game/Blueprints/BP_TheConstructor.BP_TheConstructor_C"))
  (bind _output_get (set `self.Ortho Width` (+ (* (defaults `Object` _asbp_the_constructor) 150.0) 130.0)))
  (return _output_get))

(fn `UserConstructionScript`)